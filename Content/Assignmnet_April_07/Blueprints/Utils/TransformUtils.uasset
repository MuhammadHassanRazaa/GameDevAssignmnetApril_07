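; Transform utility functions that blend an input transform toward a target transform.
; LerpTo steps toward the target with FInterpTo using delta time and a speed, while LerpToEaseInOut blends by alpha and exponent along an ease-in-out curve.
; Both interpolate each location, rotation and scale component as a separate float, so rotation blends raw Euler angles without shortest-path wrapping.
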(fn `LerpTo`
  (params (InTransform :type "Transform Structure") (TargetTransform :type "Transform Structure") (Delta :type "Float (double-precision)") (LerpRate :type "Float (double-precision)"))
  (returns (OutTransform :type "Transform Structure"))
  (return (`KismetMathLibrary.MakeTransform` (`KismetMathLibrary.MakeVector` (`KismetMathLibrary.FInterpTo` (.x (.location (`local.InTransform`))) (.x (.location (`local.TargetTransform`))) (`local.Delta`) (`local.LerpRate`)) (`KismetMathLibrary.FInterpTo` (.y (.location (`local.InTransform`))) (.y (.location (`local.TargetTransform`))) (`local.Delta`) (`local.LerpRate`)) (`KismetMathLibrary.FInterpTo` (.z (.location (`local.InTransform`))) (.z (.location (`local.TargetTransform`))) (`local.Delta`) (`local.LerpRate`))) (`KismetMathLibrary.MakeRotator` (`KismetMathLibrary.FInterpTo` (.roll (.rotation (`local.InTransform`))) (.roll (.rotation (`local.TargetTransform`))) (`local.Delta`) (`local.LerpRate`)) (`KismetMathLibrary.FInterpTo` (.pitch (.rotation (`local.InTransform`))) (.pitch (.rotation (`local.TargetTransform`))) (`local.Delta`) (`local.LerpRate`)) (`KismetMathLibrary.FInterpTo` (.yaw (.rotation (`local.InTransform`))) (.yaw (.rotation (`local.TargetTransform`))) (`local.Delta`) (`local.LerpRate`))) (`KismetMathLibrary.MakeVector` (`KismetMathLibrary.FInterpTo` (.x (.scale (`local.InTransform`))) (.x (.scale (`local.TargetTransform`))) (`local.Delta`) (`local.LerpRate`)) (`KismetMathLibrary.FInterpTo` (.y (.scale (`local.InTransform`))) (.y (.scale (`local.TargetTransform`))) (`local.Delta`) (`local.LerpRate`)) (`KismetMathLibrary.FInterpTo` (.z (.scale (`local.InTransform`))) (.z (.scale (`local.TargetTransform`))) (`local.Delta`) (`local.LerpRate`))))))

(fn `LerpToEaseInOut`
  (params (InTransform :type "Transform Structure") (TargetTransform :type "Transform Structure") (Alpha :type "Float (double-precision)") (Exponent :type "Float (double-precision)"))
  (returns (OutTransform :type "Transform Structure"))
  (return (`KismetMathLibrary.MakeTransform` (`KismetMathLibrary.MakeVector` (`KismetMathLibrary.FInterpEaseInOut` (.x (.location (`local.InTransform`))) (.x (.location (`local.TargetTransform`))) (`local.Alpha`) (`local.Exponent`)) (`KismetMathLibrary.FInterpEaseInOut` (.y (.location (`local.InTransform`))) (.y (.location (`local.TargetTransform`))) (`local.Alpha`) (`local.Exponent`)) (`KismetMathLibrary.FInterpEaseInOut` (.z (.location (`local.InTransform`))) (.z (.location (`local.TargetTransform`))) (`local.Alpha`) (`local.Exponent`))) (`KismetMathLibrary.MakeRotator` (`KismetMathLibrary.FInterpEaseInOut` (.roll (.rotation (`local.InTransform`))) (.roll (.rotation (`local.TargetTransform`))) (`local.Alpha`) (`local.Exponent`)) (`KismetMathLibrary.FInterpEaseInOut` (.pitch (.rotation (`local.InTransform`))) (.pitch (.rotation (`local.TargetTransform`))) (`local.Alpha`) (`local.Exponent`)) (`KismetMathLibrary.FInterpEaseInOut` (.yaw (.rotation (`local.InTransform`))) (.yaw (.rotation (`local.TargetTransform`))) (`local.Alpha`) (`local.Exponent`))) (`KismetMathLibrary.MakeVector` (`KismetMathLibrary.FInterpEaseInOut` (.x (.scale (`local.InTransform`))) (.x (.scale (`local.TargetTransform`))) (`local.Alpha`) (`local.Exponent`)) (`KismetMathLibrary.FInterpEaseInOut` (.y (.scale (`local.InTransform`))) (.y (.scale (`local.TargetTransform`))) (`local.Alpha`) (`local.Exponent`)) (`KismetMathLibrary.FInterpEaseInOut` (.z (.scale (`local.InTransform`))) (.z (.scale (`local.TargetTransform`))) (`local.Alpha`) (`local.Exponent`))))))