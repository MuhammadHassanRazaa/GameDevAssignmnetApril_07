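; Test_Card1 is a test card Actor Blueprint in the CardDatabase folder, with placeholder behavior for card events.
; Its OnPlace, OnDrawn and OnTaken events each print a debug string naming the card and the action.
; BeginPlay, overlap and Tick are disabled stubs, and the construction script only calls its parent.
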(event `/Game/Assignmnet_April_07/Blueprints/CardBehaviour.OnPlace`
  (`KismetSystemLibrary.PrintString` "TestCard 1 Placed"))

(event `/Game/Assignmnet_April_07/Blueprints/CardBehaviour.OnDrawn`
  (`KismetSystemLibrary.PrintString` "TestCard 1 Drawn"))

(event `/Game/Assignmnet_April_07/Blueprints/CardBehaviour.OnTaken`
  (`KismetSystemLibrary.PrintString` "TestCard 1 Taken"))

(fn `UserConstructionScript`
  (`parent.UserConstructionScript`))